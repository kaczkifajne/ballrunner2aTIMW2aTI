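; BP_crystal_01 is a spinning crystal actor that flies to the player and disappears when its collision box is overlapped.
; Tick applies a constant local rotation, and any overlap plays a timeline without checking which actor entered.
; The timeline lerps from the crystal's current location toward the player pawn's live location, so it homes in, while fading the point light to zero.
; The actor destroys itself when the timeline finishes.
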(event OnComponentBeginOverlap(box-collision)
  (params (OverlappedComponent :type Primitive%20Component%20Object%20Reference) (OtherActor :type Actor%20Object%20Reference) (OtherComp :type Primitive%20Component%20Object%20Reference) (OtherBodyIndex :type Integer) (bFromSweep :type Boolean) (SweepResult :type Hit%20Result%20Structure%20%28by%20ref%29))
  ;[0.5605 1 0.9602] crystal come
  (bind (_direction _newtrack_0 _light) (Timeline|timeline_CrystralMovement Play)
    (:Update
      (Transformation|SetActorLocation (Math|Vector|Lerp(Vector) (Transformation|GetActorLocation) (Transformation|GetActorLocation (Game|Player|GetPlayerPawn 0)) _newtrack_0) false false)
      (Rendering|Components|Light|SetIntensity (Variables|Default|GetPointLight) (Math|Float|Lerp (Variables|Default|Getlight-inte) 0.0 _light)))
    (:Finished
      (Actor|DestroyActor))))

(event EventTick
  (params (DeltaSeconds :type Float%20%28single-precision%29))
  (Transformation|AddActorLocalRotation "0,1.000000, 0" false false))

(fn ConstructionScript)