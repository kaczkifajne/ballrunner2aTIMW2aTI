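; Player-controlled ball that rolls and jumps.
; Up/Down and Left/Right axis inputs, scaled by a Multiply value, apply torque to the Sphere as an acceleration change.
; SpaceBar restarts the Jump timeline, which sets the Sphere's world location each update to the actor's location plus a scaled Z curve offset, so the jump moves it directly rather than by physics impulse.
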(event Input|AxisEvents|InputAxisUp/Down
  (params (AxisValue :type Float%20%28single-precision%29))
  ;[1 0.4858 0.5456] move mechanic
  (Class|PrimitiveComponent|AddTorqueinDegrees (Variables|Default|GetSphere) (Math|Vector|MakeVector 0.0 (* AxisValue (Variables|Default|Getmultiply)) 0.0) "None" true))

(event Input|AxisEvents|InputAxisLeft/Right
  (params (AxisValue :type Float%20%28single-precision%29))
  ;[1 0.4858 0.5456] move mechanic
  (Class|PrimitiveComponent|AddTorqueinDegrees (Variables|Default|GetSphere) (Math|Vector|MakeVector (* AxisValue (Variables|Default|Getmultiply)) 0.0 0.0) "None" true))

(event Input|KeyboardEvents|SpaceBar
  (params (Key :type Key%20Structure :default "None"))
  (bind _returnvalue (Transformation|GetActorLocation))
  ;[0.7659 1 0.7748] jump mechanic
  (:Pressed
    (bind _jump (Timeline|jump PlayFromStart)
      (:Update
        (Transformation|SetWorldLocation (Variables|Default|GetSphere) (Math|Vector|MakeVector (.x _returnvalue) (.y _returnvalue) (+ (.z _returnvalue) (* (.z _jump) 6.0))) false false)))))

(fn ConstructionScript)