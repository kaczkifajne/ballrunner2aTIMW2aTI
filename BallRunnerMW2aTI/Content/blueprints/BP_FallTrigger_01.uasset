(event OnComponentEndOverlap(FallTrigger)
  (params (OverlappedComponent :type Primitive%20Component%20Object%20Reference) (OtherActor :type Actor%20Object%20Reference) (OtherComp :type Primitive%20Component%20Object%20Reference) (OtherBodyIndex :type Integer))
  ;[1 0.519 0.5589] camera fade
  (bind _returnvalue (Game|GetCurrentLevelName true))
  (CameraFades|StartCameraFade (Variables|/Script/Engine.PlayerController|GetPlayerCameraManager (Game|GetPlayerController 0)) 0.0 1.0 0.5 "(R=0.046665,G=0.001518,B=0.004391,A=1.000000)" false false)
  (Development|PrintText "PRZEGRAŁES!!!" true true "(R=1.000000,G=0.108720,B=0.784214,A=1.000000)" 0.5)
  (Utilities|FlowControl|Delay 0.5)
  (Game|OpenLevel(byName) (Utilities|String|StringToName _returnvalue)))

(event EventBeginPlay
  ;[1 0.8906 0.8906] camera fade out
  (CameraFades|StartCameraFade (Variables|/Script/Engine.PlayerController|GetPlayerCameraManager (Game|GetPlayerController 0)) 1.0 0.0 0.5 "(R=0.031896,G=0.001214,B=0.003347,A=1.000000)" false false))

(fn ConstructionScript)