(event Collision|EventActorBeginOverlap
  (params (OtherActor :type Actor%20Object%20Reference))
  ;[1 0.06771 0.06771] kill
  (bind _returnvalue (Game|GetCurrentLevelName true))
  (CameraFades|StartCameraFade (Variables|/Script/Engine.PlayerController|GetPlayerCameraManager (Game|GetPlayerController 0)) 0.0 1.0 0.5 "(R=0.046665,G=0.001518,B=0.004391,A=1.000000)" false false)
  (Development|PrintText "PRZEGRAŁES!!!" true true "(R=1.000000,G=0.108720,B=0.784214,A=1.000000)" 0.5)
  (Utilities|FlowControl|Delay 0.5)
  (Game|OpenLevel(byName) (Utilities|String|StringToName _returnvalue)))

(event EventBeginPlay
  ;[1 1 1] Comment
  (CameraFades|StartCameraFade (Variables|/Script/Engine.PlayerController|GetPlayerCameraManager (Game|GetPlayerController 0)) 1.0 0.0 0.5 "(R=0.031896,G=0.001214,B=0.003347,A=1.000000)" false false)
  (bind _newtrack_0 (Timeline|Timeline_0 Play)
    (:Update
      (Rendering|Components|Light|SetIntensity (Variables|Default|GetPointLight) (Math|Float|Lerp (Variables|Default|Getbegin) 0.0 _newtrack_0)))))

(fn ConstructionScript)